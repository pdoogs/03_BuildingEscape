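; Openable door actor that swings around its yaw axis in response to OnOpen and OnClose from OpenDoor.
; BeginPlay caches the starting rotation, and a timeline adds its OpenAngle to it on each update.
; Opening plays the timeline and closing reverses it.
; A DoOnce is reset on open and entered on close but drives nothing, and the sound playback node never runs.
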(event `self.ReceiveBeginPlay`
  (bind _output_get (set `self.InitialRotation` (`self.K2_GetActorRotation`))))

(event `self.OpenDoor.OnOpen`
  (`|ExecutionSequence`
    (:`then_0`
      (bind (_direction _open_angle) (`Timeline|Timeline_0` :!label _label)
        (:`Update`
          (`self.K2_SetActorRotation` (`KismetMathLibrary.ComposeRotators` (stale `self.ReceiveBeginPlay` _output_get) (`KismetMathLibrary.MakeRotator` 0.0 0.0 _open_angle))))))
    (:`then_1`
      (goto _label_2 :!via `Reset`))))

(event `self.OpenDoor.OnClose`
  (`|ExecutionSequence`
    (:`then_0`
      (goto _label :!via `Reverse`))
    (:`then_1`
      (`/Engine/EditorBlueprintResources/StandardMacros.DoOnce` false :!label _label_2))))

(fn `UserConstructionScript`)